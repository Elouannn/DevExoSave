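; BP_Porte is a door that opens while the third-person character is inside its trigger box and closes when they leave.
; BeginPlay caches the starting pitch of six static meshes, which a reversible Timeline offsets together, setting their roll and yaw to zero.
; The first opening also loads a level instance from a soft reference, guarded by a DoOnce.
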(event OnComponentBeginOverlap(Box)
  (params (OverlappedComponent :type Primitive%20Component%20Object%20Reference) (OtherActor :type Actor%20Object%20Reference) (OtherComp :type Primitive%20Component%20Object%20Reference) (OtherBodyIndex :type Integer) (bFromSweep :type Boolean) (SweepResult :type Hit%20Result%20Structure%20%28by%20ref%29))
  (Utilities|Casting|CastToBP_ThirdPersonCharacter OtherActor)
  (CallFunction|OpentheDoor)
  (Utilities|FlowControl|DoOnce false
    (:Completed
      (Class|LevelStreamingDynamic|LoadLevelInstancebySoftObjectPtr (Variables|Default|GetLevel) "0, 0, 0" "0, 0, 0" "" 0 false))))

(event OnComponentEndOverlap(Box)
  (params (OverlappedComponent :type Primitive%20Component%20Object%20Reference) (OtherActor :type Actor%20Object%20Reference) (OtherComp :type Primitive%20Component%20Object%20Reference) (OtherBodyIndex :type Integer))
  (Utilities|Casting|CastToBP_ThirdPersonCharacter OtherActor)
  (CallFunction|ClosetheDoor))

(event Custom|Open%20The%20door
  (bind _newtrack_0 (Timeline|Timeline Play)
    (:Update
      (for (_array_element _array_index) (Variables|Default|GetArray)
        (Transformation|SetRelativeRotation _array_element (Math|Rotator|MakeRotator 0.0 (- (Utilities|Array|Get(acopy) (Variables|Default|GetBaseYCoordinate) _array_index) _newtrack_0) 0.0) false false)))))

(event Custom|CloseTheDoor
  (bind _newtrack_0 (Timeline|Timeline Reverse)
    (:Update
      (for (_array_element _array_index) (Variables|Default|GetArray)
        (Transformation|SetRelativeRotation _array_element (Math|Rotator|MakeRotator 0.0 (- (Utilities|Array|Get(acopy) (Variables|Default|GetBaseYCoordinate) _array_index) _newtrack_0) 0.0) false false)))))

(event EventBeginPlay
  (bind _output_get (Variables|Default|SetArray (Utilities|Array|MakeArray (Variables|Default|GetStaticMesh1) (Variables|Default|GetStaticMesh2) (Variables|Default|GetStaticMesh3) (Variables|Default|GetStaticMesh4) (Variables|Default|GetStaticMesh5) (Variables|Default|GetStaticMesh))))
  (for _array_element _output_get
    (Utilities|Array|Add (Variables|Default|GetBaseYCoordinate) (.pitch (Variables|/Script/Engine.SceneComponent|GetRelativeRotation _array_element)))))

(fn ConstructionScript)