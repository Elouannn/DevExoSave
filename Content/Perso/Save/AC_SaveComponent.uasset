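; AC_SaveComponent is a save component that creates, saves, loads, deletes and checks BP_SaveGame slots.
; ActualGameData holds the active save object, created with a default name and player ID or cast from the loaded slot.
; Save, load and delete use SlotName with user index 0, while the existence check uses ActualGameData's SaveFileName and PlayerID.
; LoadSave ignores its Async input and loads synchronously.
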(fn SaveGame
  (SaveGame|SaveGametoSlot (Variables|Default|GetActualGameData) (Variables|Default|GetSlot%20Name)))

(fn LoadSave
  (params (Async :type Boolean))
  (bind _returnvalue (SaveGame|LoadGamefromSlot (Variables|Default|GetSlot%20Name)))
  (bind _asbp_save_game (Utilities|Casting|CastToBP_SaveGame _returnvalue))
  (Variables|Default|SetActualGameData _asbp_save_game)
  (Math|Integer|IncrementInt (Variables|Default|GetTestInteger)
    (:%20%20
      (Variables|Default|SetTestInteger 0))))

(fn CreateSave
  (bind _returnvalue (SaveGame|CreateSaveGameObject "/Game/Perso/Save/BP_SaveGame.BP_SaveGame_C"))
  (Variables|Default|SetActualGameData _returnvalue)
  (Variables|/Game/Perso/Save/BP_SaveGame.BP_SaveGame_C|SetPlayerID (Variables|Default|GetActualGameData) 0)
  (Variables|/Game/Perso/Save/BP_SaveGame.BP_SaveGame_C|SetSaveFileName (Variables|Default|GetActualGameData) "DefaultName")
  (return))

(fn DeleteSave
  (SaveGame|DeleteGameinSlot (Variables|Default|GetSlot%20Name)))

(fn CheckExistingSave
  (bind _actualgamedata (Variables|Default|GetActualGameData))
  (bind _returnvalue (SaveGame|DoesSaveGameExist (Variables|/Game/Perso/Save/BP_SaveGame.BP_SaveGame_C|GetSaveFileName _actualgamedata) (Variables|/Game/Perso/Save/BP_SaveGame.BP_SaveGame_C|GetPlayerID _actualgamedata)))
  (return _returnvalue))