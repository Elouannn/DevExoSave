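; BP_Quest is a quest Blueprint that registers itself with the game's quest manager and marks its quest as started.
; On BeginPlay it gets the QuestManager from GI_GameInstance, presents itself, and has the manager load data for its DataAssetRef.
; It then prints the quest's Started flag and sets it to true, writing runtime state directly on the referenced data asset.
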(event Custom|ApplyData
  (bind _dataassetref (Variables|Default|GetDataAssetRef))
  (Development|PrintString (Utilities|String|Append "The quest is actually Started ? " (Utilities|String|ToString(Boolean) (Variables|/Game/MesBP/Data/DataAssetQuest.DataAssetQuest_C|GetStarted _dataassetref))))
  (Variables|/Game/MesBP/Data/DataAssetQuest.DataAssetQuest_C|SetStarted _dataassetref true))

(event EventBeginPlay
  (bind _asgi_game_instance (Utilities|Casting|CastToGI_GameInstance (Game|GetGameInstance)))
  (bind _output_get (Variables|Default|SetReferent (Variables|/Game/MesBP/CustomActors/GI_GameInstance.GI_GameInstance_C|GetQuestManager _asgi_game_instance)))
  (Default|PresentYourself _output_get self)
  (Default|LoadData _output_get (Variables|Default|GetDataAssetRef))
  (CallFunction|ApplyData))

(fn ConstructionScript)