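; BP_QuestManager is a quest manager that starts quests and resets their progress.
; On BeginPlay it registers itself on GI_GameInstance, then calls LoadData, which is an empty stub here.
; AddQuest marks a quest as started if it is neither completed nor already started.
; ResetAllQuest restores the completed, name and started fields of every entry in AllQuests from its stored base values.
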(event Custom|ResetAllQuest
  (for _array_element (Variables|Default|GetAllQuests)
    (Variables|/Game/MesBP/Data/StructDA_Quests.StructDA_Quests_C|SetCompleted _array_element (Variables|/Game/MesBP/Data/StructDA_Quests.StructDA_Quests_C|GetBaseCompleted _array_element))
    (Variables|/Game/MesBP/Data/StructDA_Quests.StructDA_Quests_C|SetName _array_element (Variables|/Game/MesBP/Data/StructDA_Quests.StructDA_Quests_C|GetBaseName _array_element))
    (Variables|/Game/MesBP/Data/StructDA_Quests.StructDA_Quests_C|SetStarted _array_element (Variables|/Game/MesBP/Data/StructDA_Quests.StructDA_Quests_C|GetBaseStarted _array_element))))

(event Custom|AddQuest
  (params (NewQuest :type Struct%20DA%20Quests%20Object%20Reference))
  (if (not (Variables|/Game/MesBP/Data/StructDA_Quests.StructDA_Quests_C|GetCompleted NewQuest))
    (if (not (Variables|/Game/MesBP/Data/StructDA_Quests.StructDA_Quests_C|GetStarted NewQuest))
      (Variables|/Game/MesBP/Data/StructDA_Quests.StructDA_Quests_C|SetStarted NewQuest true))))

(event Custom|LoadData)

(event EventBeginPlay
  (bind _asgi_game_instance (Utilities|Casting|CastToGI_GameInstance (Game|GetGameInstance)))
  (Variables|Default|SetGameInstance _asgi_game_instance)
  (Variables|/Game/MesBP/CustomActors/GI_GameInstance.GI_GameInstance_C|SetQuestManager (Variables|Default|GetGameInstance) self)
  (CallFunction|LoadData))

(fn ConstructionScript)