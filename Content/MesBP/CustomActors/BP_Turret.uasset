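; BP_Turret is a turret the player takes over on Interact, with the player controller possessing it to aim and fire.
; Look input rotates a horizontal pivot with free yaw and clamped pitch.
; Shoot input passes a gate that acts as a short cooldown, then ChoseGun cycles through four cannons to pick the bullet's spawn transform.
; A timeline animates the firing cannon along X; the muzzle FX toggles are unwired.
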(event Input|EnhancedActionEvents|EnhancedInputActionIA_Shoot
  (params (ActionValue :type Boolean) (ElapsedSeconds :type Float%20%28double-precision%29) (TriggeredSeconds :type Float%20%28double-precision%29) (InputAction :type Input%20Action%20Object%20Reference :default "/Game/FirstPerson/Input/Actions/IA_Shoot.IA_Shoot"))
  (Utilities|FlowControl|Gate false :!label _label
    (:Exit
      (Utilities|FlowControl|Sequence
        (:then_0
          (goto _label Close))
        (:then_1
          (Utilities|FlowControl|Delay 0.3)
          (goto _label Open))
        (:then_2
          (bind (_bulletspawntarget _shootingcanon _fxtoshoot) (CallFunction|ChoseGun))
          (Game|SpawnActorfromClass "/Game/MesBP/CustomActors/BP_Bullet.BP_Bullet_C" (Math|Transform|MakeTransform (.Location (Math|Transform|BreakTransform _bulletspawntarget)) (.Rotation (Math|Transform|BreakTransform _bulletspawntarget)) "1.000000,1.000000,1.000000") "Undefined" "MultiplyWithRoot" 0 0)
          (Utilities|FlowControl|Sequence
            (:then_1
              (Variables|Default|SetTempLocation (Variables|/Script/Engine.SceneComponent|GetRelativeLocation _shootingcanon))
              (bind _newtrack_0 (Timeline|Timeline PlayFromStart)
                (:Update
                  (Transformation|SetRelativeLocation _shootingcanon (Math|Vector|MakeVector (+ _newtrack_0 (.x (Variables|Default|GetTempLocation))) (.y (Variables|Default|GetTempLocation)) (.z (Variables|Default|GetTempLocation))) false false))))))))))

(event Input|EnhancedActionEvents|EnhancedInputActionIA_Look
  (params (ActionValue :type Vector%202D%20Structure) (ElapsedSeconds :type Float%20%28double-precision%29) (TriggeredSeconds :type Float%20%28double-precision%29) (InputAction :type Input%20Action%20Object%20Reference :default "/Game/FirstPerson/Input/Actions/IA_Look.IA_Look"))
  (bind _pivothoriz (Variables|Usefull|GetPivotHoriz))
  (bind _returnvalue (Transformation|GetWorldRotation _pivothoriz))
  (Transformation|SetWorldRotation _pivothoriz (Math|Rotator|MakeRotator 0.0 (Math|Float|Clamp(Float) (+ (.pitch _returnvalue) (* (.y ActionValue) -1.0)) -3e+01 3e+01) (+ (.x ActionValue) (.yaw _returnvalue))) false false))

(event EventInteract
  (bind _returnvalue (Game|GetPlayerController 0))
  (Pawn|UnPossess _returnvalue)
  (bind _asbp_first_person_player_controller (Utilities|Casting|CastToBP_FirstPersonPlayerController _returnvalue))
  (Pawn|Possess _asbp_first_person_player_controller self))

(fn ConstructionScript)

(fn ChoseGun
  (if (== (Variables|Usefull|GetCanonShooting) 4)
    (Variables|Usefull|SetCanonShooting 0))
  (switch int (Variables|Usefull|GetCanonShooting)
    (:Default
      (Variables|Usefull|SetBullet%20Spawn%20Target (Transformation|GetWorldTransform (Variables|Default|GetStaticMesh3)) :!label _label)
      (Variables|Usefull|SetFXTo%20Shoot (Variables|Default|GetExplo2))
      (Variables|Usefull|SetShootingCanon (Variables|Construct|GetGun1)))
    (:0
      (goto _label))
    (:1
      (Variables|Usefull|SetBullet%20Spawn%20Target (Transformation|GetWorldTransform (Variables|Default|GetStaticMesh2)))
      (Variables|Usefull|SetFXTo%20Shoot (Variables|Default|GetExplo3))
      (Variables|Usefull|SetShootingCanon (Variables|Construct|GetGun2)))
    (:2
      (Variables|Usefull|SetBullet%20Spawn%20Target (Transformation|GetWorldTransform (Variables|Default|GetStaticMesh1)))
      (Variables|Usefull|SetFXTo%20Shoot (Variables|Default|GetExplo1))
      (Variables|Usefull|SetShootingCanon (Variables|Construct|GetGun3)))
    (:3
      (Variables|Usefull|SetBullet%20Spawn%20Target (Transformation|GetWorldTransform (Variables|Default|GetStaticMesh)))
      (Variables|Usefull|SetFXTo%20Shoot (Variables|Default|GetExplo))
      (Variables|Usefull|SetShootingCanon (Variables|Construct|GetGun4))))
  (Variables|Usefull|SetCanonShooting (+ (Variables|Usefull|GetCanonShooting) 1))
  (return (Variables|Usefull|GetBullet%20Spawn%20Target) (Variables|Usefull|GetShootingCanon) (Variables|Usefull|GetFXTo%20Shoot)))