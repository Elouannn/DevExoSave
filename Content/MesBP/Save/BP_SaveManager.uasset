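; Save manager that persists quest progress to a single BP_SaveGame slot and registers itself on GI_GameInstance at BeginPlay.
; SaveGame copies the QuestManager's quest data assets and flattens their Completed and Started flags into parallel arrays before writing.
; Saving and loading create a fresh save object when no slot exists.
; LoadSave only caches the loaded object as ActualGameData, without applying it back to quests.
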(event EventBeginPlay
  (bind _asgi_game_instance (Utilities|Casting|CastToGI_GameInstance (Game|GetGameInstance)))
  (Variables|/Game/MesBP/CustomActors/GI_GameInstance.GI_GameInstance_C|SetSaveManager _asgi_game_instance self))

(fn ConstructionScript)

(fn CreateSave
  (bind _returnvalue (SaveGame|CreateSaveGameObject "/Game/MesBP/Save/BP_SaveGame.BP_SaveGame_C"))
  (Variables|Default|SetActualGameData _returnvalue)
  (return))

(fn CheckExistingSave
  (bind _returnvalue (SaveGame|DoesSaveGameExist "DefaultValue"))
  (return _returnvalue))

(fn LoadSave
  (bind _exist (CallFunction|CheckExistingSave))
  (if _exist
    _
    (else
      (CallFunction|CreateSave)))
  (bind _returnvalue (SaveGame|LoadGamefromSlot "DefaultValue"))
  (bind _asbp_save_game (Utilities|Casting|CastToBP_SaveGame _returnvalue))
  (Variables|Default|SetActualGameData _asbp_save_game)
  (return))

(fn SaveGame
  (bind _exist (CallFunction|CheckExistingSave))
  (if _exist
    _
    (else
      (CallFunction|CreateSave)))
  ;[1 1 1] SaveQuest
  (bind _output_get (Variables|/Game/MesBP/Save/BP_SaveGame.BP_SaveGame_C|SetAllQuests (Variables|Default|GetActualGameData) (Variables|/Game/MesBP/Quests/BP_QuestManager.BP_QuestManager_C|GetAllQuestsDA (Variables|Default|GetQuestManager))))
  (CallFunction|GetAllQuestResult _output_get)
  (SaveGame|SaveGametoSlot (Variables|Default|GetActualGameData) "DefaultValue")
  (return))

(fn GetAllQuestResult
  (params (NewParam :type Array%20of%20Data%20Asset%20Quest%20Object%20References))
  (bind _actualgamedata (Variables|Default|GetActualGameData))
  (bind _completed (Variables|/Game/MesBP/Save/BP_SaveGame.BP_SaveGame_C|GetCompleted _actualgamedata))
  (bind _started (Variables|/Game/MesBP/Save/BP_SaveGame.BP_SaveGame_C|GetStarted _actualgamedata))
  (Utilities|Array|Clear _completed)
  (Utilities|Array|Clear _started)
  (for _array_element NewParam
    (Utilities|Array|Add _completed (Variables|/Game/MesBP/Data/DataAssetQuest.DataAssetQuest_C|GetCompleted _array_element))
    (Utilities|Array|Add _started (Variables|/Game/MesBP/Data/DataAssetQuest.DataAssetQuest_C|GetStarted _array_element)))
  (return))